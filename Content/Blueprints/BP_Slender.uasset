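; Slender spawner that repeatedly makes a BP_ThirdPersonCharacter appear around the player for a random time, then destroys it.
; A BeginPlay delay loop drives spawning at random offsets within a distance range, with the character's yaw turned toward the player.
; Spawn points come from retried debug-drawn sphere traces that look for actors tagged Terrain.
; A second downward trace from high above then sets the character on the ground using its capsule half-height.
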(event `self.ReceiveBeginPlay`
  (`KismetSystemLibrary.Delay` (`KismetMathLibrary.RandomFloatInRange` (`self.MinSpawnTime`) (`self.MaxSpawnTime`)) :!label _label)
  (bind _slender (`self.SpawnCharacterAtRandomLocation`))
  (if (`KismetSystemLibrary.IsValid` _slender)
    (bind (_returnvalue_x _returnvalue_y) (`KismetMathLibrary.BreakVector` (`self.K2_GetActorLocation` _slender)))
    (bind _returnvalue (`KismetMathLibrary.MakeVector` _returnvalue_x _returnvalue_y (+ 0.0 10000.0)))
    (bind _corrected_position (`self.GetValidTerrainCollision` 5.0 _returnvalue (+ _returnvalue (* (* (`self.GetActorUpVector` _slender) -1.0) 15000.0)) true _slender))
    (`self.K2_SetActorLocation` _slender _corrected_position false false)
    (`KismetSystemLibrary.Delay` (`KismetMathLibrary.RandomFloatInRange` (`self.MinDespawnTime`) (`self.MaxDespawnTime`)))
    (`self.K2_DestroyActor` _slender) ; Destroy Slender And Spawn Again
    (goto _label)
    (else
      (goto _label))))

(event `self.ReceiveTick`
  (params (DeltaSeconds :type "Float (single-precision)")))

(fn `GetValidSpawnPosition`
  (returns (`Spawn Position` :type "Vector Structure"))
  (bind _returnvalue (`KismetMathLibrary.RandomFloatInRange` (`self.MinDistance`) (`self.MaxDistance`)))
  (bind _returnvalue_2 (`KismetMathLibrary.DegreesToRadians` (`KismetMathLibrary.RandomFloatInRange` 0.0 360.0)))
  (bind _returnvalue_3 (+ (`KismetMathLibrary.MakeVector` (* (`KismetMathLibrary.Cos` _returnvalue_2) _returnvalue) (* _returnvalue (`KismetMathLibrary.Sin` _returnvalue_2))) (`SceneComponent.K2_GetComponentLocation` (`Character.Mesh` (`GameplayStatics.GetPlayerCharacter` 0)))))
  (for _ (range 16)
    (bind (_corrected_position _terrain_collision) (`self.GetValidTerrainCollision` 30.0 (+ _returnvalue_3 (0.0 0.0 1000.0)) (- _returnvalue_3 (0.0 0.0 1000.0))))
    (if _terrain_collision
      (`KismetSystemLibrary.LogString` "Right Position")
      (break)
      (else
        (`KismetSystemLibrary.LogString` "Corrected"))))
  (return _corrected_position))

(fn `GetValidTerrainCollision`
  (params (`Sphere Radius` :type "Float (double-precision)") (Start :type "Vector Structure") (End :type "Vector Structure") (`Correct Spawn` :type Boolean) (Actor :type "Actor Object Reference"))
  (returns (`Corrected Position` :type "Vector Structure") (`Terrain Collision` :type Boolean))
  (bind (_returnvalue_x _returnvalue_y) (`KismetMathLibrary.BreakVector` (`SceneComponent.K2_GetComponentLocation` (`Actor.RootComponent` Actor))))
  (bind (_outhit _returnvalue) (`KismetSystemLibrary.SphereTraceSingleForObjects` :`Start` Start :`End` End :`Radius` `Sphere Radius` :`ObjectTypes` (`|MakeArray` "ObjectTypeQuery1" "ObjectTypeQuery2" "ObjectTypeQuery4" :!type "EObjectTypeQuery Enum") :`DrawDebugType` "ForDuration"))
  (if _returnvalue
    (bind (_bblockinghit _binitialoverlap _time _distance _location _impactpoint _normal _impactnormal _physmat _hitactor) (`GameplayStatics.BreakHitResult` _outhit))
    (bind _returnvalue_2 (`self.ActorHasTag` _hitactor "Terrain"))
    (if _returnvalue_2
      (if `Correct Spawn`
        (return (`KismetMathLibrary.MakeVector` _returnvalue_x _returnvalue_y (+ (.z _impactpoint) (`CapsuleComponent.CapsuleHalfHeight` (`self.GetComponentByClass` Actor "/Script/Engine.CapsuleComponent")))) _returnvalue_2)
        (else
          (return (`KismetMathLibrary.MakeVector` (.x _impactpoint) (.y _impactpoint) (.z _impactpoint)) _returnvalue_2))))))

(fn `SpawnCharacterAtRandomLocation`
  (returns (Slender :type "Actor Object Reference"))
  (bind _spawn_position (`self.GetValidSpawnPosition`))
  (bind _returnvalue (`|SpawnActorFromClass` "/Game/ThirdPerson/Blueprints/BP_ThirdPersonCharacter.BP_ThirdPersonCharacter_C" (`KismetMathLibrary.Conv_VectorToTransform` _spawn_position) "Undefined" "MultiplyWithRoot" null null))
  (set `self.Slender` _returnvalue)
  (bind _slender (`self.Slender`)
    (:`then`
      (bind _rootcomponent (`Actor.RootComponent` _slender))
      (bind (_returnvalue_roll _returnvalue_pitch) (`KismetMathLibrary.BreakRotator` (`SceneComponent.K2_GetComponentRotation` _rootcomponent)))
      (bind (_returnvalue_roll_2 _returnvalue_pitch_2 _returnvalue_yaw) (`KismetMathLibrary.BreakRotator` (`KismetMathLibrary.FindLookAtRotation` (`SceneComponent.K2_GetComponentLocation` _rootcomponent) (`SceneComponent.K2_GetComponentLocation` (`Character.Mesh` (`GameplayStatics.GetPlayerCharacter` 0))))))
      (`SceneComponent.K2_SetWorldRotation` _rootcomponent (`KismetMathLibrary.MakeRotator` _returnvalue_roll _returnvalue_pitch _returnvalue_yaw) false false)
      (return _slender))
    (:`else`)))

(fn `UserConstructionScript`)