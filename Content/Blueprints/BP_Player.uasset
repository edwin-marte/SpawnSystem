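; Player Blueprint for a Slender game that detects whether Slender is in the player's view.
; On BeginPlay it caches the first BP_Slender actor as SlenderAI.
; Each Tick, IsSlenderInCameraView validates that AI's Slender actor, projects its location to screen, checks viewport bounds and requires line of sight from the camera.
; The result drives nothing yet, as the branch is empty and the debug logs are disconnected.
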(event `Slender Reference`
  (bind _outactors (`GameplayStatics.GetAllActorsOfClass` "/Game/Blueprints/BP_Slender.BP_Slender_C"))
  (set `self.SlenderAI` (`|GetArrayItem` _outactors)))

(event `self.ReceiveBeginPlay`
  (`self.Slender Reference`))

(event `self.ReceiveTick`
  (params (DeltaSeconds :type "Float (single-precision)"))
  (bind _incameraview (`self.IsSlenderInCameraView`))
  (if _incameraview
    _))

(fn `IsSlenderInCameraView`
  (returns (InCameraView :type Boolean))
  (bind _returnvalue (`GameplayStatics.GetPlayerController` 0))
  (bind (_returnvalue_x _returnvalue_y) (`KismetMathLibrary.BreakVector2D` (`WidgetLayoutLibrary.GetViewportSize`)))
  (bind _slender (`/Game/Blueprints/BP_Slender.Slender` (`self.SlenderAI`)))
  (bind _screenlocation (`PlayerController.ProjectWorldLocationToScreen` (`GameplayStatics.GetPlayerController` 0) (`self.K2_GetActorLocation` _slender) false))
  ;[1 1 1] Check Bounds
  (if (`KismetSystemLibrary.IsValid` _slender)
    (return (and (and (> (`KismetMathLibrary.BreakVector2D` _screenlocation) 0.0) (> (`.Y` (`KismetMathLibrary.BreakVector2D` _screenlocation)) 0.0) (< (`KismetMathLibrary.BreakVector2D` _screenlocation) _returnvalue_x) (< (`.Y` (`KismetMathLibrary.BreakVector2D` _screenlocation)) _returnvalue_y)) (`Controller.LineOfSightTo` _returnvalue (`/Game/Blueprints/BP_Slender.Slender` (`self.SlenderAI`)) (`SceneComponent.K2_GetComponentLocation` (`PlayerCameraManager.TransformComponent` (`PlayerController.PlayerCameraManager` _returnvalue))) false)))))

(fn `UserConstructionScript`)